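; Base dialogue component that opens a W_Dialogue widget and drives branching conversations through an empty Dialogue function, presumably overridden by children.
; Each choice is stored in the DialogueProgress map, then Dialogue reruns from the start.
; AddDialogue increments the index and either returns a stored option (looked up at key 0) or updates the widget.
; Helpers clear or trim stored progress.
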(event EventBeginPlay)

(event EventTick
  (params (DeltaSeconds :type Float%20%28single-precision%29)))

(fn OpenConversation
  (bind _returnvalue (UserInterface|CreateWidget "/Game/UI/W_Dialogue.W_Dialogue_C" 0 self))
  (bind _output_get (Variables|Default|SetDialogue%20Widget _returnvalue))
  (UserInterface|Viewport|AddtoViewport _output_get 0)
  (CallFunction|ProgressDialogue))

(fn CloseDialogue
  (Widget|RemovefromParent (Variables|Default|GetDialogue%20Widget)))

(fn ProgressDialogue
  (Variables|Default|SetDialogue%20Index -1)
  (CallFunction|Dialogue))

(fn Dialogue)

(fn AddDialogue
  (params (Speaker :type Text) (Dialogue :type Text) (Options :type Array%20of%20Texts))
  (bind _dialogue_progress (Variables|Default|GetDialogue%20Progress))
  (bind (_value _returnvalue) (Utilities|Map|Find _dialogue_progress 0))
  (Math|Integer|IncrementInt (Variables|Default|GetDialogue%20Index)
    (:%20%20
      (if _returnvalue
        (return "NewEnumerator0" _value)
        (else
          (Default|UpdateDialogueText (Variables|Default|GetDialogue%20Widget) (Variables|Default|GetDialogue%20Index) Speaker Dialogue Options)
          (return "NewEnumerator1" 0))))))

(fn UpdateSelectedOption
  (params (Progress%20Index%20 :type Integer) (Option%20Index :type Integer))
  (Utilities|Map|Add (Variables|Default|GetDialogue%20Progress) Progress%20Index%20 Option%20Index)
  (CallFunction|ProgressDialogue))

(fn ClearDialogueProgress
  (Utilities|Map|Clear (Variables|Default|GetDialogue%20Progress)))

(fn RemoveDialogueProgress
  (params (Progress%20Steps :type Integer))
  (for _index (range 0 Progress%20Steps)
    (Utilities|Map|Remove (Variables|Default|GetDialogue%20Progress) (- (stale _output_get) _index)))
  (bind _output_get (Variables|Default|SetDialogue%20Index 0)))

(fn SetDialogueTreeIndex
  (CallFunction|SetDialogueTreeIndex)
  (CallFunction|ClearDialogueProgress))
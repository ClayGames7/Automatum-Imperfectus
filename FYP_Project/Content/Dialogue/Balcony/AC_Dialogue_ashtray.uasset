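; AC_Dialogue_ashtray is the dialogue script for an inspectable ashtray in the Balcony dialogue set, voiced by the ashtray, skill voices and the player.
; The Dialogue override calls its parent, then chains AddDialogue nodes through their Pass Through states, with Encyclopaedia and Electrochemistry interjections using hard-coded check labels.
; A final choice accepts or refuses the nicotine craving, and both branches end by clearing progress and closing dialogue, with no task logic.
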(event EventBeginPlay
  (|CallParentFunction) ; This node is disabled and will not be called.\nDrag off pins to build functionality.
)

(event EventTick
  (params (DeltaSeconds :type Float%20%28single-precision%29))
  (|CallParentFunction DeltaSeconds) ; This node is disabled and will not be called.\nDrag off pins to build functionality.
)

(fn Dialogue
  (|CallParentFunction)
  (bind _state (CallFunction|AddDialogue "Ashtray" "Ashtray - A soot covered ashtray, three recently lit C-Stick Butts , underneath lies a faded and blurred Logo can only be seen as 'De___mp C___et__'" (Utilities|Array|MakeArray "")))
  (switch Utilities|FlowControl|Switch|SwitchonE_DialogueBase _state
    (:NewEnumerator0
      (bind _state_2 (CallFunction|AddDialogue "Encyclopaedia" "[Medium:Sucess] - The company that made this Ashtray is a relatively small company called Deschamps Ciggarette Trays. They were successful for a strong 6 Months before Comp Holdings saw the success, made their own and nearly instantly bankrupted the company" (Utilities|Array|MakeArray "")))
      (switch Utilities|FlowControl|Switch|SwitchonE_DialogueBase _state_2
        (:NewEnumerator0
          (bind (_state_3 _option_index_) (CallFunction|AddDialogue "Electrochemistry" " [Trivial:Success] - YUMMY... You need some more, I can still taste that sweet succulent nicotine in our teeth, buy more, buy more, buy moooreeeee" (Utilities|Array|MakeArray "1. - \"God I can feel the sweat, I need another one\" (Accept Task)" "2. - No... I can't, I gotta stop. ")))
          (switch Utilities|FlowControl|Switch|SwitchonE_DialogueBase _state_3
            (:NewEnumerator0
              (switch int _option_index_
                (:0
                  (bind (_state_4 _option_index__2) (CallFunction|AddDialogue "Electrochemistry" " YESSSSS... the only shops that sell the GOOOOD stuff is on the lowest levels. next time we are there. GET ONE." (Utilities|Array|MakeArray "[LEAVE]")))
                  (switch Utilities|FlowControl|Switch|SwitchonE_DialogueBase _state_4
                    (:NewEnumerator0
                      (switch int _option_index__2
                        (:0
                          (CallFunction|ClearDialogueProgress)
                          (CallFunction|CloseDialogue))))))
                (:1
                  (bind (_state_5 _option_index__3) (CallFunction|AddDialogue "You" "2. - No... I can't, I gotta stop." (Utilities|Array|MakeArray "[LEAVE]")))
                  (switch Utilities|FlowControl|Switch|SwitchonE_DialogueBase _state_5
                    (:NewEnumerator0
                      (switch int _option_index__3
                        (:0
                          (CallFunction|ClearDialogueProgress)
                          (CallFunction|CloseDialogue))))))))))))))
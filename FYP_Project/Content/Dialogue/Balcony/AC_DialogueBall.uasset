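; Balcony dialogue component for an ancient football, a branching comic scene where the player can leave it, pop it or attempt a bicycle kick.
; The Dialogue override calls its parent, then chains AddDialogue nodes by State and OptionIndex, with skills as speakers.
; Skill check results and morale changes are hardcoded text, with no rolls or stat updates.
; Endings clear progress and close the dialogue, except the "Owww!" branch.
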(fn Dialogue
  (|CallParentFunction)
  (bind (_state _option_index_) (CallFunction|AddDialogue "Ball" "A football, Looks ancient. Like something from the old world." (Utilities|Array|MakeArray "")))
  (switch Utilities|FlowControl|Switch|SwitchonE_DialogueBase _state
    (:NewEnumerator0
      (switch int _option_index_
        (:Default
          (bind (_state_2 _option_index__2) (CallFunction|AddDialogue "Encyclopaedia" "[Easy:Success] - More Specifically, this is from the year 2023, just over a decde after this city was founded, created in the then empire of New North" (Utilities|Array|MakeArray "1. - \"Hmm... I wonder why I have this? Anyway I should get the Door\"" "2. - Embrace the chaos and destroy ball" "3. - [Hand/Eye Coordinantion - Medium 12] Start doing Keepy Ups")))
          (switch Utilities|FlowControl|Switch|SwitchonE_DialogueBase _state_2
            (:NewEnumerator0
              (switch int _option_index__2
                (:0
                  (bind (_state_3 _option_index__3) (CallFunction|AddDialogue "You" "1. - \"Hmm... I wonder why I have this? Anyway I should get the Door\"" (Utilities|Array|MakeArray "[LEAVE]")))
                  (switch Utilities|FlowControl|Switch|SwitchonE_DialogueBase _state_3
                    (:NewEnumerator0
                      (switch int _option_index__3
                        (:0
                          (CallFunction|ClearDialogueProgress)
                          (CallFunction|CloseDialogue))))))
                (:1
                  (bind (_state_4 _option_index__4) (CallFunction|AddDialogue "You" "Ball - BANG! a loud Pop destroys the ball. Why you did this to an artifact like that is unknown, but it made you happy. 
Plus 1 MORALE" (Utilities|Array|MakeArray "[LEAVE]")))
                  (switch Utilities|FlowControl|Switch|SwitchonE_DialogueBase _state_4
                    (:NewEnumerator0
                      (switch int _option_index__4
                        (:0
                          (CallFunction|ClearDialogueProgress)
                          (CallFunction|CloseDialogue))))))
                (:2
                  (bind (_state_5 _option_index__5) (CallFunction|AddDialogue "Hand/Eye Coordination" "Pop, Pop, Pow. each beautiful bounce off your knees and feet, reminiscent of the incredible Thierry Messindo." (Utilities|Array|MakeArray "")))
                  (switch Utilities|FlowControl|Switch|SwitchonE_DialogueBase _state_5
                    (:NewEnumerator0
                      (switch int _option_index__5
                        (:0
                          (bind (_state_6 _option_index__6) (CallFunction|AddDialogue "Physical Instrument" "YOU SHOULD DO A BICYCLE KICK" (Utilities|Array|MakeArray "")))
                          (switch Utilities|FlowControl|Switch|SwitchonE_DialogueBase _state_6
                            (:NewEnumerator0
                              (switch int _option_index__6
                                (:0
                                  (bind (_state_7 _option_index__7) (CallFunction|AddDialogue "Logic" "You absolutely cannot do it, you're a middle aged man with a dad bod who hasn't even entered a gym since he was 18, let alone ever kicked a ball" (Utilities|Array|MakeArray "1. - [Hand/Eye Coordinantion - Medium 12]  Go for the bicycle kick with flair!!" "2. - Set the ball down \"No... I absolutely should not do this\" ")))
                                  (switch Utilities|FlowControl|Switch|SwitchonE_DialogueBase _state_7
                                    (:NewEnumerator0
                                      (switch int _option_index__7
                                        (:0
                                          (bind (_state_8 _option_index__8) (CallFunction|AddDialogue "Hand/Eye Coordination" "[medium:Success] - The arc, the brilliant curve and stunning pose, all in mid air, this is almost a miracle! 
-> Miracle" (Utilities|Array|MakeArray "1. - [Physical Instrument - Medium 12]  belt the ball across the sky Powerfully!")))
                                          (switch Utilities|FlowControl|Switch|SwitchonE_DialogueBase _state_8
                                            (:NewEnumerator0
                                              (switch int _option_index__8
                                                (:0
                                                  (bind (_state_9 _option_index__9) (CallFunction|AddDialogue "Hand/Eye Coordination" "[Medium:Failure] - despite the grace, and effort, you try so hard to strike the ball with force unlike any other... But you overshot it and end up landing tits up on your back, incredible failure, hope someone recorded it 
Neagtive 1 MORALE" (Utilities|Array|MakeArray "")))
                                                  (switch Utilities|FlowControl|Switch|SwitchonE_DialogueBase _state_9
                                                    (:NewEnumerator0
                                                      (switch int _option_index__9
                                                        (:0
                                                          (bind (_state_10 _option_index__10) (CallFunction|AddDialogue "Logic" "Told you" (Utilities|Array|MakeArray "1. - \"Owww!\"" "2. - \"Ow, I bet that was cool... ow\"")))
                                                          (switch Utilities|FlowControl|Switch|SwitchonE_DialogueBase _state_10
                                                            (:NewEnumerator0
                                                              (switch int _option_index__10
                                                                (:0
                                                                  (bind (_state_11 _option_index__11) (CallFunction|AddDialogue "You" "1. - \"Owww!\"" (Utilities|Array|MakeArray "[LEAVE]")))
                                                                  (switch Utilities|FlowControl|Switch|SwitchonE_DialogueBase _state_11
                                                                    (:NewEnumerator0
                                                                      (switch int _option_index__11))))
                                                                (:1
                                                                  (bind (_state_12 _option_index__12) (CallFunction|AddDialogue "Logic" "It was not" (Utilities|Array|MakeArray "[LEAVE]")))
                                                                  (switch Utilities|FlowControl|Switch|SwitchonE_DialogueBase _state_12
                                                                    (:NewEnumerator0
                                                                      (switch int _option_index__12
                                                                        (:0
                                                                          (CallFunction|ClearDialogueProgress)
                                                                          (CallFunction|CloseDialogue))))))))))))))))))
                                        (:1
                                          (bind (_state_13 _option_index__13) (CallFunction|AddDialogue "You" "2. - Set the ball down \"No... I absolutely should not do this\"" (Utilities|Array|MakeArray "[LEAVE]")))
                                          (switch Utilities|FlowControl|Switch|SwitchonE_DialogueBase _state_13
                                            (:NewEnumerator0
                                              (switch int _option_index__13
                                                (:0
                                                  (CallFunction|ClearDialogueProgress)
                                                  (CallFunction|CloseDialogue))))))))))))))))))))))))))
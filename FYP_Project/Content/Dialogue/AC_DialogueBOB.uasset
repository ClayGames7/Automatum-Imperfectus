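; Dialogue component for the character Bob, defining a short branching conversation with crude lines and player reply options.
; The Dialogue override calls its parent, then uses AddDialogue to show Bob's opening question with two replies.
; When that node's state is Pass Through, the chosen option index selects one of two follow-up lines, each with two replies that lead nowhere further.
; A switch on DialogueTreeIndex has no cases.
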(event EventBeginPlay
  (|CallParentFunction) ; This node is disabled and will not be called.\nDrag off pins to build functionality.
)

(event EventTick
  (params (DeltaSeconds :type Float%20%28single-precision%29))
  (|CallParentFunction DeltaSeconds) ; This node is disabled and will not be called.\nDrag off pins to build functionality.
)

(fn Dialogue
  (|CallParentFunction)
  (switch int (Variables|Default|GetDialogue%20Tree%20Index)
    (:0
      (bind (_state _option_index_) (CallFunction|AddDialogue "Bob" "Do you want to have fuck with me?" (Utilities|Array|MakeArray "What" "eww")))
      (switch Utilities|FlowControl|Switch|SwitchonE_DialogueBase _state
        (:NewEnumerator0
          (switch int _option_index_
            (:0
              (CallFunction|AddDialogue "Bob" "I said Do you want to have fuck with me?" (Utilities|Array|MakeArray "Are you okay?" "no thank you")))
            (:1
              (CallFunction|AddDialogue "Bob" "Do you think I'm gross...." (Utilities|Array|MakeArray "yes" "no ")))))))))
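; Dialogue component for the test-level NPC Ashtray, also labeled Bill, holding a branching conversation about the player's identity.
; The Dialogue override calls its parent, then nests AddDialogue calls, branching on each returned State and OptionIndex.
; RemoveDialogueProgress rewinds retry branches, while endings call ClearDialogueProgress and CloseDialogue.
; The P.I. route includes a skill-tagged Suggestion option, with no check here, that points to brother Bob.
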(event EventBeginPlay
  (|CallParentFunction) ; This node is disabled and will not be called.\nDrag off pins to build functionality.
)

(event EventTick
  (params (DeltaSeconds :type Float%20%28single-precision%29))
  (|CallParentFunction DeltaSeconds) ; This node is disabled and will not be called.\nDrag off pins to build functionality.
)

(fn Dialogue
  (|CallParentFunction)
  (|CallParentFunction)
  (bind (_state _option_index_) (CallFunction|AddDialogue "Ashtray" "Hey there! I'm Ashtray, who are you?" (Utilities|Array|MakeArray "I Don't know my name" "i'm a ... P.I." "I am the looming death that will inhabit all")))
  (switch Utilities|FlowControl|Switch|SwitchonE_DialogueBase _state
    (:NewEnumerator0
      (switch int _option_index_
        (:0
          (bind (_state_2 _option_index__2) (CallFunction|AddDialogue "Ashtray" "That's sad... but sometimes I don't know my name, but I'm bill" (Utilities|Array|MakeArray "Hi Ashtray" "I don't care")))
          (switch Utilities|FlowControl|Switch|SwitchonE_DialogueBase _state_2
            (:NewEnumerator0
              (switch int _option_index__2
                (:0
                  (CallFunction|RemoveDialogueProgress 2))
                (:1
                  (bind (_state_3 _option_index__3) (CallFunction|AddDialogue "Ashtray" "That's mean, you're a meanie" (Utilities|Array|MakeArray "I don't care" "I'm sorry")))
                  (switch Utilities|FlowControl|Switch|SwitchonE_DialogueBase _state_3
                    (:NewEnumerator0
                      (switch int _option_index__3
                        (:0
                          (bind (_state_4 _option_index__4) (CallFunction|AddDialogue "Ashtray" "LEAVE ME ALONE!!" (Utilities|Array|MakeArray "[Leave]")))
                          (switch Utilities|FlowControl|Switch|SwitchonE_DialogueBase _state_4
                            (:NewEnumerator0
                              (switch int _option_index__4
                                (:0
                                  (CallFunction|ClearDialogueProgress)
                                  (CallFunction|CloseDialogue))))))
                        (:1
                          (bind (_state_5 _option_index__5) (CallFunction|AddDialogue "Ashtray" "It's okay, let's try again!" (Utilities|Array|MakeArray "Okay kid" "No")))
                          (switch Utilities|FlowControl|Switch|SwitchonE_DialogueBase _state_5
                            (:NewEnumerator0
                              (switch int _option_index__5
                                (:0
                                  (CallFunction|RemoveDialogueProgress 3))
                                (:1
                                  (CallFunction|ClearDialogueProgress)
                                  (CallFunction|CloseDialogue))))))))))))))
        (:1
          (bind (_state_6 _option_index__6) (CallFunction|AddDialogue "Ashtray" "Hi mr P.I. guy! are you here to interview me?" (Utilities|Array|MakeArray "No" "[Suggestion - Easy8 ] - why, do you have something to tell me? ")))
          (switch Utilities|FlowControl|Switch|SwitchonE_DialogueBase _state_6
            (:NewEnumerator0
              (switch int _option_index__6
                (:0
                  (CallFunction|AddDialogue "Ashtray" "Oh then bye bye!?" (Utilities|Array|MakeArray "[Leave]"))
                  (CallFunction|ClearDialogueProgress)
                  (CallFunction|CloseDialogue))
                (:1
                  (bind (_state_7 _option_index__7) (CallFunction|AddDialogue "Bill" "Then you should probably talk to my brother Bob... he's weird and scares me, be careful" (Utilities|Array|MakeArray "Thanks Bill [Leave]")))
                  (switch Utilities|FlowControl|Switch|SwitchonE_DialogueBase _state_7
                    (:NewEnumerator0
                      (switch int _option_index__7
                        (:0
                          (CallFunction|ClearDialogueProgress)
                          (CallFunction|CloseDialogue))))))))))
        (:2
          (bind (_state_8 _option_index__8) (CallFunction|AddDialogue "Bill" "Hey mr  looming death that will inhabit all, that's a scary name" (Utilities|Array|MakeArray "You're weird" "The world will crumble under capitalist destruction")))
          (switch Utilities|FlowControl|Switch|SwitchonE_DialogueBase _state_8
            (:NewEnumerator0
              (switch int _option_index__8
                (:0
                  (bind (_state_9 _option_index__9) (CallFunction|AddDialogue "Bill" "That's mean, you're a meanie" (Utilities|Array|MakeArray "I don't care" "I'm sorry")))
                  (switch Utilities|FlowControl|Switch|SwitchonE_DialogueBase _state_9
                    (:NewEnumerator0
                      (switch int _option_index__9
                        (:0
                          (bind (_state_10 _option_index__10) (CallFunction|AddDialogue "Bill" "LEAVE ME ALONE!!" (Utilities|Array|MakeArray "[Leave]")))
                          (switch Utilities|FlowControl|Switch|SwitchonE_DialogueBase _state_10
                            (:NewEnumerator0
                              (switch int _option_index__10
                                (:0
                                  (CallFunction|ClearDialogueProgress)
                                  (CallFunction|CloseDialogue))))))
                        (:1
                          (bind (_state_11 _option_index__11) (CallFunction|AddDialogue "Bill" "It's okay, let's try again!" (Utilities|Array|MakeArray "Okay kid" "No")))
                          (switch Utilities|FlowControl|Switch|SwitchonE_DialogueBase _state_11
                            (:NewEnumerator0
                              (switch int _option_index__11
                                (:0
                                  (CallFunction|RemoveDialogueProgress 2))
                                (:1
                                  (CallFunction|ClearDialogueProgress)
                                  (CallFunction|CloseDialogue))))))))))
                (:1
                  (bind (_state_12 _option_index__12) (CallFunction|AddDialogue "Bill" "Ooo what's a capitalist?" (Utilities|Array|MakeArray "A cancer" "Nice people, we should bend our working knees to them")))
                  (switch Utilities|FlowControl|Switch|SwitchonE_DialogueBase _state_12
                    (:NewEnumerator0
                      (switch int _option_index__12
                        (:0
                          (bind (_state_13 _option_index__13) (CallFunction|AddDialogue "Bill" "Oh... that's bad... I hate capitalists! let's burn them all" (Utilities|Array|MakeArray "Good Kid")))
                          (switch Utilities|FlowControl|Switch|SwitchonE_DialogueBase _state_13
                            (:NewEnumerator0
                              (switch int _option_index__13
                                (:0
                                  (CallFunction|ClearDialogueProgress)
                                  (CallFunction|CloseDialogue))))))
                        (:1
                          (bind (_state_14 _option_index__14) (CallFunction|AddDialogue "Bill" "That's good... I love capitalists! we should not burn them all" (Utilities|Array|MakeArray "Good Kid")))
                          (switch Utilities|FlowControl|Switch|SwitchonE_DialogueBase _state_14
                            (:NewEnumerator0
                              (switch int _option_index__14
                                (:0
                                  (CallFunction|ClearDialogueProgress)
                                  (CallFunction|CloseDialogue))))))))))))))))))
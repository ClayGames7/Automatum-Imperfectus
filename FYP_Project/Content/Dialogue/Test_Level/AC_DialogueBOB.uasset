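; Dialogue component for Bob, a Test_Level character who crudely propositions the player through branching conversations.
; Overrides Dialogue and switches on DialogueTreeIndex between a first-meeting tree and a return-visit tree, nesting AddDialogue calls by chosen option.
; Endings close the dialogue after either setting the tree index for next time or clearing progress.
; One branch instead calls RemoveDialogueProgress to step back within the conversation.
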(event EventBeginPlay
  (|CallParentFunction) ; This node is disabled and will not be called.\nDrag off pins to build functionality.
)

(event EventTick
  (params (DeltaSeconds :type Float%20%28single-precision%29))
  (|CallParentFunction DeltaSeconds) ; This node is disabled and will not be called.\nDrag off pins to build functionality.
)

(fn Dialogue
  (|CallParentFunction)
  (switch int (Variables|Default|GetDialogue%20Tree%20Index)
    (:0
      (bind (_state _option_index_) (CallFunction|AddDialogue "Bob" "Do you want to have fuck with me I know you do, I know you love me, love me please?" (Utilities|Array|MakeArray "What" "eww")))
      (switch Utilities|FlowControl|Switch|SwitchonE_DialogueBase _state
        (:NewEnumerator0
          (switch int _option_index_
            (:0
              (bind (_state_2 _option_index__2) (CallFunction|AddDialogue "Bob" "I said Do you want to have fuck with me?" (Utilities|Array|MakeArray "okay. go for it" "no thank you")))
              (switch Utilities|FlowControl|Switch|SwitchonE_DialogueBase _state_2
                (:NewEnumerator0
                  (switch int _option_index__2
                    (:0
                      (bind (_state_3 _option_index__3) (CallFunction|AddDialogue "Bob" "Goooood, come back when you want some mclovin" (Utilities|Array|MakeArray "[Leave]")))
                      (switch Utilities|FlowControl|Switch|SwitchonE_DialogueBase _state_3
                        (:NewEnumerator0
                          (switch int _option_index__3
                            (:0
                              (CallFunction|SetDialogueTreeIndex 1)
                              (CallFunction|CloseDialogue))))))
                    (:1
                      (bind (_state_4 _option_index__4) (CallFunction|AddDialogue "Bob" "your loss" (Utilities|Array|MakeArray "[Leave]")))
                      (switch Utilities|FlowControl|Switch|SwitchonE_DialogueBase _state_4
                        (:NewEnumerator0
                          (switch int _option_index__4
                            (:0
                              (CallFunction|ClearDialogueProgress)
                              (CallFunction|CloseDialogue))))))))))
            (:1
              (bind (_state_5 _option_index__5) (CallFunction|AddDialogue "Bob" "Do you think I'm gross...." (Utilities|Array|MakeArray "yes I do" "no, of course not ")))
              (switch Utilities|FlowControl|Switch|SwitchonE_DialogueBase _state_5
                (:NewEnumerator0
                  (switch int _option_index__5
                    (:0
                      (bind (_state_6 _option_index__6) (CallFunction|AddDialogue "Bob" "Then Bugger off" (Utilities|Array|MakeArray "[Leave]")))
                      (switch Utilities|FlowControl|Switch|SwitchonE_DialogueBase _state_6
                        (:NewEnumerator0
                          (switch int _option_index__6
                            (:0
                              (CallFunction|ClearDialogueProgress)
                              (CallFunction|CloseDialogue))))))
                    (:1
                      (bind (_state_7 _option_index__7) (CallFunction|AddDialogue "Bob" "In that case..." (Utilities|Array|MakeArray "Yes?")))
                      (switch Utilities|FlowControl|Switch|SwitchonE_DialogueBase _state_7
                        (:NewEnumerator0
                          (switch int _option_index__7
                            (:0
                              (CallFunction|RemoveDialogueProgress 2))))))))))))))
    (:1
      (bind (_state_8 _option_index__8) (CallFunction|AddDialogue "Bob" "Are you here for some McLovin?" (Utilities|Array|MakeArray "Yes I am" "ahaha i lied" "Let me think about it")))
      (switch Utilities|FlowControl|Switch|SwitchonE_DialogueBase _state_8
        (:NewEnumerator0
          (switch int _option_index__8
            (:0
              (bind (_state_9 _option_index__9) (CallFunction|AddDialogue "Bob" "PAHAHAHAHA HOW DESPERATE ARE YOU AHAHAH" (Utilities|Array|MakeArray "Ouch" "so is your mum")))
              (switch Utilities|FlowControl|Switch|SwitchonE_DialogueBase _state_9
                (:NewEnumerator0
                  (switch int _option_index__9
                    (:0
                      _)
                    (:1
                      _))
                  (CallFunction|SetDialogueTreeIndex 1)
                  (CallFunction|CloseDialogue))))
            (:1
              (bind (_state_10 _option_index__10) (CallFunction|AddDialogue "Bob" "God, you are just detestable... I like that, come back when you change your mind" (Utilities|Array|MakeArray "[Leave]")))
              (switch Utilities|FlowControl|Switch|SwitchonE_DialogueBase _state_10
                (:NewEnumerator0
                  (switch int _option_index__10
                    (:0
                      (CallFunction|SetDialogueTreeIndex)
                      (CallFunction|CloseDialogue))))))
            (:2
              (bind (_state_11 _option_index__11) (CallFunction|AddDialogue "Bob" "Then Bugger off until you know" (Utilities|Array|MakeArray "[Leave]")))
              (switch Utilities|FlowControl|Switch|SwitchonE_DialogueBase _state_11
                (:NewEnumerator0
                  (switch int _option_index__11
                    (:0
                      (CallFunction|ClearDialogueProgress)
                      (CallFunction|CloseDialogue))))))))))))
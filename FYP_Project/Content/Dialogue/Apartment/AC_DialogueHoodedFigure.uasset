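; Dialogue component for the Hooded Figure in the apartment, who pitches a serial-killer case to the player's amnesiac private investigator.
; The overridden Dialogue function switches on DialogueTreeIndex and chains AddDialogue calls, branching on OptionIndex, with several side paths rejoining the main pitch.
; Skill voices interject with check results written into the text rather than rolled.
; Refusing the cult lead sets index 1 for a return greeting; several branches, including most acceptances, have no follow-up.
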(event EventBeginPlay
  (|CallParentFunction) ; This node is disabled and will not be called.\nDrag off pins to build functionality.
)

(event EventTick
  (params (DeltaSeconds :type Float%20%28single-precision%29))
  (|CallParentFunction DeltaSeconds) ; This node is disabled and will not be called.\nDrag off pins to build functionality.
)

(fn Dialogue
  (|CallParentFunction)
  (switch int (Variables|Default|GetDialogue%20Tree%20Index)
    (:0
      (bind (_state _option_index_) (CallFunction|AddDialogue "The Hooded Figure " "A Thin sillhouette shrowded in the darkness waits intently for you to speak." (Utilities|Array|MakeArray "")))
      (switch Utilities|FlowControl|Switch|SwitchonE_DialogueBase _state
        (:NewEnumerator0
          (switch int _option_index_
            (:0
              (bind (_state_2 _option_index__2) (CallFunction|AddDialogue "Volition " "[Easy:Success] - This shadow stands with such gravity, a strong sense of pride in him, You've got this, make the opening, keep it professional" (Utilities|Array|MakeArray "")))
              (switch Utilities|FlowControl|Switch|SwitchonE_DialogueBase _state_2
                (:NewEnumerator0
                  (switch int _option_index__2
                    (:0
                      (bind (_state_3 _option_index__3) (CallFunction|AddDialogue "Esperit De Corps " " [Medium:Fail] - This man exudes so much authority, so much gravitas, who is he? " (Utilities|Array|MakeArray "1. - \"Hi there, I am... I am the Owner of this agency\"" "2. - \"Who are you? why are you here?\" (Asked only If you failed the Check) " "3. - Try and Ignore him and leave calmly and cooly")))
                      (switch Utilities|FlowControl|Switch|SwitchonE_DialogueBase _state_3
                        (:NewEnumerator0
                          (switch int _option_index__3
                            (:0
                              (bind (_state_4 _option_index__4) (CallFunction|AddDialogue "The Hooded Figure" "\"It's a pleasure to make your aquiantance, I have been waiting for a while, unsteady area to loiter this place is, but I've heard you are the best of the best in this abyss-forsaken city\" He fiddles with his hands like an Actor shuffling a script." (Utilities|Array|MakeArray "1. - \"The City is really and truly shit, for the past week, all I've heard is the screams coming from the lowest reaches\"" "2. - \"The best? Glad to hear that, I had no idea, Truthfully I can't remember much\"")))
                              (switch Utilities|FlowControl|Switch|SwitchonE_DialogueBase _state_4
                                (:NewEnumerator0
                                  (switch int _option_index__4
                                    (:0
                                      (bind (_state_5 _option_index__5) (CallFunction|AddDialogue "The Hooded Figure " "A faint smile brekas from the vignette of his hooded carapace \"Yes, Yes Yes. So you see it too? Hear it too? the way this City pains and troubles, a cancer feeds on this city\"" (Utilities|Array|MakeArray "") :!label _label))
                                      (switch Utilities|FlowControl|Switch|SwitchonE_DialogueBase _state_5
                                        (:NewEnumerator0
                                          (switch int _option_index__5
                                            (:0
                                              (bind (_state_6 _option_index__6) (CallFunction|AddDialogue "The Hooded Figure " "The Smile fades immediately, in the blink of an eye his face stares, Icy and harsh. \"Let's be real here Mr. Von Hart... This city, much like the Smog Filled Meadows of Northern Fallan is riddled with crime, corruption and wars. Not to mention *The Workers* gaining a new lease on life as it were\"" (Utilities|Array|MakeArray "")))
                                              (switch Utilities|FlowControl|Switch|SwitchonE_DialogueBase _state_6
                                                (:NewEnumerator0
                                                  (switch int _option_index__6
                                                    (:0
                                                      (bind (_state_7 _option_index__7) (CallFunction|AddDialogue "Composure " "[Medium:Fail] - He is running circles around our brain, This is too much for only being here a week... 
DAMAGED MORALE -1" (Utilities|Array|MakeArray "1. - \"Please Slow down, this is too much to understand... Hangover Y'know\"")))
                                                      (switch Utilities|FlowControl|Switch|SwitchonE_DialogueBase _state_7
                                                        (:NewEnumerator0
                                                          (switch int _option_index__7
                                                            (:0
                                                              (bind (_state_8 _option_index__8) (CallFunction|AddDialogue "The Hooded Figure " "he steps closer, and whispers in the ear, imperceptable to anyone were they in this room \"they were slaves and nothing more, they knew this, their purpose, they have base emotions but no emotional range like you or I, they cannot reproduce, they do not truly bleed or breathe\"." (Utilities|Array|MakeArray "")))
                                                              (switch Utilities|FlowControl|Switch|SwitchonE_DialogueBase _state_8
                                                                (:NewEnumerator0
                                                                  (switch int _option_index__8
                                                                    (:0
                                                                      (bind (_state_9 _option_index__9) (CallFunction|AddDialogue "The Hooded Figure " " \"But yet... here we are, many have went against the grain, revolted and have made their way into society, illegaly, It's commendable and truly respectable, their drive to survive.\"" (Utilities|Array|MakeArray "1. - \"What Does this have to do with me? (Continue)" "2. - [Conceptualisation - Easy 8] “What Do you think of their dreams then?”")))
                                                                      (switch Utilities|FlowControl|Switch|SwitchonE_DialogueBase _state_9
                                                                        (:NewEnumerator0
                                                                          (switch int _option_index__9
                                                                            (:0
                                                                              _)
                                                                            (:1
                                                                              (bind (_state_10 _option_index__10) (CallFunction|AddDialogue "The Hooded Figure " "No movement through the abyss under the overhanging hood “Do machines dream?”" (Utilities|Array|MakeArray "1. - “How can we know? I dream”" "2. - \"Let's just go back on track... why are you here?\" (Continue)")))
                                                                              (switch Utilities|FlowControl|Switch|SwitchonE_DialogueBase _state_10
                                                                                (:NewEnumerator0
                                                                                  (switch int _option_index__10
                                                                                    (:0
                                                                                      (bind (_state_11 _option_index__11) (CallFunction|AddDialogue "The Hooded Figure " "“Are you flesh and blood?” The shadow asks in excitedly as he lifts his head up to look at the P.I from now on, no longer avoiding his gaze. " (Utilities|Array|MakeArray "1. -  \"I… I don’t Know, I can’t remember\"." "2. - \"No... no more, let's just get to the matter at hand\" (Continue)")))
                                                                                      (switch Utilities|FlowControl|Switch|SwitchonE_DialogueBase _state_11
                                                                                        (:NewEnumerator0
                                                                                          (switch int _option_index__11
                                                                                            (:0
                                                                                              (bind (_state_12 _option_index__12) (CallFunction|AddDialogue "The Hooded Figure " " “Does anyone truly remember? Are our thoughts just given to us from those at the top, the Companies that dictate life, I mean we are but ants to SafeView right?” A deepening Grin, twitches in each word, subtle voice breaks, Taking a drink of a flask, offereing some to The P.I. to no acknowledgement." (Utilities|Array|MakeArray "")))
                                                                                              (switch Utilities|FlowControl|Switch|SwitchonE_DialogueBase _state_12
                                                                                                (:NewEnumerator0
                                                                                                  (switch int _option_index__12
                                                                                                    (:0
                                                                                                      _)))))
                                                                                            (:1
                                                                                              _)))))
                                                                                    (:1
                                                                                      _))))))
                                                                          (bind (_state_13 _option_index__13) (CallFunction|AddDialogue "The Hooded Figure" "“Anyway, the real reason I am here... Mr Von Hart, have you heard of the butcherings that have been occuring every week for 3 months? Been nonstop news reports on it here, 'The Most Prolific Serial Killer in Sun's Dawn History' as they say\"" (Utilities|Array|MakeArray "1. - \"Can't say that I have? Not really a news guy\"" "2. - \"Think I heard it on the radio outside? The church cult?\"" "3. - \" I think I know where you're going here, I'm a P.I. not a detective, you want me to see if your wife is cheating? I'm your guy, but chasing killers? Nah\"") :!label _label_2))
                                                                          (switch Utilities|FlowControl|Switch|SwitchonE_DialogueBase _state_13
                                                                            (:NewEnumerator0
                                                                              (switch int _option_index__13
                                                                                (:0
                                                                                  (bind (_state_14 _option_index__14) (CallFunction|AddDialogue "The Hooded Figure" "“I see, Given your condition I don't blame you. News is just fearmongering and Propaganda, but this... this is serious and the news doesn't take it as such; That's why I'm here.\"" (Utilities|Array|MakeArray "")))
                                                                                  (switch Utilities|FlowControl|Switch|SwitchonE_DialogueBase _state_14
                                                                                    (:NewEnumerator0
                                                                                      (switch int _option_index__14
                                                                                        (:0
                                                                                          (bind (_state_15 _option_index__15) (CallFunction|AddDialogue "The Hooded Figure" "“Each murder has been getting worse and more brazen, each act is in public display like a damned puzzle. A sign. A message. I need to know as to whom this message is for, and for it to stop\"" (Utilities|Array|MakeArray "")))
                                                                                          (switch Utilities|FlowControl|Switch|SwitchonE_DialogueBase _state_15
                                                                                            (:NewEnumerator0
                                                                                              (switch int _option_index__15
                                                                                                (:0
                                                                                                  (bind (_state_16 _option_index__16) (CallFunction|AddDialogue "Drama" "[Medium:Success] - ahh a thrilling murder mystery, I love this, who is the killer? You... Me... THE CONTRACT ISSUER?? this is my favourite intro, Feels like we are Holming Watts 'Detective extraodinaire'!!!\"" (Utilities|Array|MakeArray "")))
                                                                                                  (switch Utilities|FlowControl|Switch|SwitchonE_DialogueBase _state_16
                                                                                                    (:NewEnumerator0
                                                                                                      (switch int _option_index__16
                                                                                                        (:0
                                                                                                          (bind (_state_17 _option_index__17) (CallFunction|AddDialogue "Shivers" "[Medium:Success] - Down on the depths of the city, through the hailstorm of bullets led by gangs and revolutionaries, amidst Prostitutes sellingt their body, Sex shop Neon polluting the sky and the latest new Swerve Hip/Hop blaring noisily through every street... A slink of a holster shrieks quietly, ready to toil in its craft. Mordaciously the fervour of this act, a malignant act of torture and defilement, shadowed away from any prying eyes. As an artistic message the body will be uncovered within the next hours, a message of symbolism..." (Utilities|Array|MakeArray "")))
                                                                                                          (switch Utilities|FlowControl|Switch|SwitchonE_DialogueBase _state_17
                                                                                                            (:NewEnumerator0
                                                                                                              (switch int _option_index__17
                                                                                                                (:0
                                                                                                                  (bind (_state_18 _option_index__18) (CallFunction|AddDialogue "Shivers" " A message to the masses above, the gods who ignore the plebes who beg for help and aid... beg to survive." (Utilities|Array|MakeArray "")))
                                                                                                                  (switch Utilities|FlowControl|Switch|SwitchonE_DialogueBase _state_18
                                                                                                                    (:NewEnumerator0
                                                                                                                      (switch int _option_index__18
                                                                                                                        (:0
                                                                                                                          (bind (_state_19 _option_index__19) (CallFunction|AddDialogue "Shivers" "But God isn't hearing the plea." (Utilities|Array|MakeArray "")))
                                                                                                                          (switch Utilities|FlowControl|Switch|SwitchonE_DialogueBase _state_19
                                                                                                                            (:NewEnumerator0
                                                                                                                              (switch int _option_index__19
                                                                                                                                (:0
                                                                                                                                  (bind (_state_20 _option_index__20) (CallFunction|AddDialogue "Shivers" "This is no heaven." (Utilities|Array|MakeArray "")))
                                                                                                                                  (switch Utilities|FlowControl|Switch|SwitchonE_DialogueBase _state_20
                                                                                                                                    (:NewEnumerator0
                                                                                                                                      (switch int _option_index__20
                                                                                                                                        (:0
                                                                                                                                          (bind (_state_21 _option_index__21) (CallFunction|AddDialogue "The Hooded Figure" "“You see Mr. Von Hart, The Faulty Ports over at SDPD haven't cared about this from the beginning and the SafeView Security don't believe this is worth their time.\"" (Utilities|Array|MakeArray "")))
                                                                                                                                          (switch Utilities|FlowControl|Switch|SwitchonE_DialogueBase _state_21
                                                                                                                                            (:NewEnumerator0
                                                                                                                                              (switch int _option_index__21
                                                                                                                                                (:0
                                                                                                                                                  (bind (_state_22 _option_index__22) (CallFunction|AddDialogue "The Hooded Figure" "“You see Mr. Von Hart, The Faulty Ports over at SDPD haven't cared about this from the beginning and the SafeView Security don't believe this is worth their time.\"" (Utilities|Array|MakeArray "")))
                                                                                                                                                  (switch Utilities|FlowControl|Switch|SwitchonE_DialogueBase _state_22
                                                                                                                                                    (:NewEnumerator0
                                                                                                                                                      (switch int _option_index__22
                                                                                                                                                        (:0
                                                                                                                                                          (bind (_state_23 _option_index__23) (CallFunction|AddDialogue "Logic" "Logic [Trivial:Success] - Nobody cares about the low district" (Utilities|Array|MakeArray "1. - \"I see, this is intriguing, Tell me more, I'm in\"" "2. - \"So, You're telling me the SDPD won't even bother and you expect me to?\"" "3. - \"Faulty Ports? That's new, I like that, will definitely use that one\"")))
                                                                                                                                                          (switch Utilities|FlowControl|Switch|SwitchonE_DialogueBase _state_23
                                                                                                                                                            (:NewEnumerator0
                                                                                                                                                              (switch int _option_index__23
                                                                                                                                                                (:2
                                                                                                                                                                  (bind (_state_24 _option_index__24) (CallFunction|AddDialogue "The Hooded Figure" "\"Great\" You can practically hear his eyes rolling \"Now please give me an answer\"" (Utilities|Array|MakeArray "1. - \"I see, this is intriguing, Tell me more, I'm in\"" "2. - \"So, You're telling me the SDPD won't even bother and you expect me to?\"")))
                                                                                                                                                                  (switch Utilities|FlowControl|Switch|SwitchonE_DialogueBase _state_24
                                                                                                                                                                    (:NewEnumerator0
                                                                                                                                                                      (switch int _option_index__24))))))))))))))))))))))))))))))))))))))))))))
                                                                                (:1
                                                                                  (bind (_state_25 _option_index__25) (CallFunction|AddDialogue "The Hooded Figure" "“You've heard right. it's the leading theory that the cult you've heard about *The followers of the Swallowing Darkness* are behind this. Gruesome dispays to showcase their beliefs that the worlds death is upon them, thanks to the *Gaping Mouth*\"" (Utilities|Array|MakeArray "")))
                                                                                  (switch Utilities|FlowControl|Switch|SwitchonE_DialogueBase _state_25
                                                                                    (:NewEnumerator0
                                                                                      (switch int _option_index__25
                                                                                        (:0
                                                                                          (bind (_state_26 _option_index__26) (CallFunction|AddDialogue "The Hooded Figure" "“Truthfully I don't know much else about them, but yes, they're the lead of this case but they're practicaly untouchable, being seen as an offical religioun, and that's why I need you, You can investigate this case from behind the scenes.\"" (Utilities|Array|MakeArray "1. - \"This church; it's name even evokes evil... I agree... I'll help\" " "2. - \"No... No I can't help...\" (LEAVE)")))
                                                                                          (switch Utilities|FlowControl|Switch|SwitchonE_DialogueBase _state_26
                                                                                            (:NewEnumerator0
                                                                                              (switch int _option_index__26
                                                                                                (:1
                                                                                                  (CallFunction|SetDialogueTreeIndex 1)
                                                                                                  (CallFunction|CloseDialogue))))))))))
                                                                                (:2
                                                                                  (bind (_state_27 _option_index__27) (CallFunction|AddDialogue "The Hooded Figure" "a thunderous boom from an authorative voice bellows “Don't be a damned graces grouch, listen to me, This is bigger than that. if you had a soul, empathy, you'd take the job. If this doesn't persuade you... you'll have a good price for uncovering the truth behind this... Nu-Ken, that's all you wnat right?\"" (Utilities|Array|MakeArray "")))
                                                                                  (switch Utilities|FlowControl|Switch|SwitchonE_DialogueBase _state_27
                                                                                    (:NewEnumerator0
                                                                                      (switch int _option_index__27))))))))))))))))))))))))))
                                    (:1
                                      (bind (_state_28 _option_index__28) (CallFunction|AddDialogue "The Hooded Figure " "\"Ahh, had too much synth-whisky? Been there, hard days, hard life, I understand. But yes, me and my buddies from the ground levels keep hearing of you! The greatest P.I. in Sun's Dawn\"" (Utilities|Array|MakeArray "1. - \"Yeah... drinking, that's probably it.\"" "2. - \"No, see I just woke up like this a week ago, and forgot everything\"")))
                                      (switch Utilities|FlowControl|Switch|SwitchonE_DialogueBase _state_28
                                        (:NewEnumerator0
                                          (switch int _option_index__28
                                            (:0
                                              (bind (_state_29 _option_index__29) (CallFunction|AddDialogue "The Hooded Figure " "The sillhouette Shuffles and a small cough reverberates through the hood... an uncomfortable silence fills the air" (Utilities|Array|MakeArray "")))
                                              (switch Utilities|FlowControl|Switch|SwitchonE_DialogueBase _state_29
                                                (:NewEnumerator0
                                                  (switch int _option_index__29))))
                                            (:1
                                              (bind (_state_30 _option_index__30) (CallFunction|AddDialogue "The Hooded Figure " "\"You forgot hmm, strange. Maybe a side effect of the abyssofarms that pass by this building? SafeView like always, ignoring the little man, Corporate Greed am I right?\"" (Utilities|Array|MakeArray "1. - \"AbyssoFarm?\"" "2. - stare blankly, don't say anything (Continue)" "3. - [Rhetoric - Medium 10] \"Fuck Yeah, Eat The Rich, fuck the corpos\" *Raise hand for High Five*")))
                                              (switch Utilities|FlowControl|Switch|SwitchonE_DialogueBase _state_30
                                                (:NewEnumerator0
                                                  (switch int _option_index__30
                                                    (:0
                                                      (bind (_state_31 _option_index__31) (CallFunction|AddDialogue "The Hooded Figure " "\"Much like the Steel mills of Fallan producing Abyssal Energy, thanks to the bastards of *EZ Fuel Corp*, SafeView have developed Flying Titans which develop farms which produce Synthetic Vegetables at the same time as Abyssal Energy into our atmosphere\"" (Utilities|Array|MakeArray "")))
                                                      (switch Utilities|FlowControl|Switch|SwitchonE_DialogueBase _state_31
                                                        (:NewEnumerator0
                                                          (switch int _option_index__31
                                                            (:0
                                                              (bind (_state_32 _option_index__32) (CallFunction|AddDialogue "The Hooded Figure " "\"But they've won all lawsuits somehow, shoot a holodart at an answer and It's probaly correct... But there's no proof\"" (Utilities|Array|MakeArray "")))
                                                              (switch Utilities|FlowControl|Switch|SwitchonE_DialogueBase _state_32
                                                                (:NewEnumerator0
                                                                  (switch int _option_index__32
                                                                    (:0
                                                                      (bind (_state_33 _option_index__33) (CallFunction|AddDialogue "The Hooded Figure " "\"Now tell me... do you See the cancer that this city is?\"" (Utilities|Array|MakeArray "1. - \"Yes... I see it\"" "2. - \"no, I can't say I do\"")))
                                                                      (switch Utilities|FlowControl|Switch|SwitchonE_DialogueBase _state_33
                                                                        (:NewEnumerator0
                                                                          (switch int _option_index__33
                                                                            (:0
                                                                              (goto _label))
                                                                            (:1
                                                                              (bind (_state_34 _option_index__34) (CallFunction|AddDialogue "The Hooded Figure " "“Fine, Not worth the debate If you don't see, Let's move on\"" (Utilities|Array|MakeArray "")))
                                                                              (switch Utilities|FlowControl|Switch|SwitchonE_DialogueBase _state_34
                                                                                (:NewEnumerator0
                                                                                  (switch int _option_index__34
                                                                                    (:0
                                                                                      (goto _label_2))))))))))))))))))
                                                    (:2
                                                      (bind (_state_35 _option_index__35) (CallFunction|AddDialogue "Rhetoric" "[Medium:Fail] With the smarmiest fce and most weasly gesture, even you don't convince yourself in this, you work up the muster to meakly say... \"\"Y...Yeah, Eat The Rich, f... the corpos\" *Slightly Raise hand for High Five*" (Utilities|Array|MakeArray "")))
                                                      (switch Utilities|FlowControl|Switch|SwitchonE_DialogueBase _state_35
                                                        (:NewEnumerator0
                                                          (switch int _option_index__35
                                                            (:0
                                                              (bind (_state_36 _option_index__36) (CallFunction|AddDialogue "The Hooded Figure " "\"No...\"" (Utilities|Array|MakeArray "")))
                                                              (switch Utilities|FlowControl|Switch|SwitchonE_DialogueBase _state_36
                                                                (:NewEnumerator0
                                                                  (switch int _option_index__36
                                                                    (:0
                                                                      (bind (_state_37 _option_index__37) (CallFunction|AddDialogue "The Hooded Figure " "\"Anyway...\"" (Utilities|Array|MakeArray "")))
                                                                      (switch Utilities|FlowControl|Switch|SwitchonE_DialogueBase _state_37
                                                                        (:NewEnumerator0
                                                                          (switch int _option_index__37
                                                                            (:0
                                                                              (goto _label_2))))))))))))))))))))))))))
                            (:1
                              (bind (_state_38 _option_index__38) (CallFunction|AddDialogue "The Hooded Figure" "“My name is unimportant, but who are you Mr. Van Hart? ahh it doesn't matter, we have important business. Drink? No. ahaha, you seem as though someones bypassed your synapses, loosen up, You're the P.I here\"" (Utilities|Array|MakeArray "")))
                              (switch Utilities|FlowControl|Switch|SwitchonE_DialogueBase _state_38
                                (:NewEnumerator0
                                  (switch int _option_index__38
                                    (:0
                                      (goto _label_2))))))
                            (:2
                              (bind (_state_39 _option_index__39) (CallFunction|AddDialogue "Drama " "[Medium:Success] - \"If you're gonna just leave him, why not let his mind be full of bliss, give him the upmost adoration of our story. He is probably nobody important anyway so use fancy words you don't even know the words for\"" (Utilities|Array|MakeArray "1. - [Drama - Medium 10] \"There's a Huge datacrash over on Turin Street and they need me to retriangulate the code, you should come by in another parsec!\"" "2. - Leave without saying anything [LEAVE]")))
                              (switch Utilities|FlowControl|Switch|SwitchonE_DialogueBase _state_39
                                (:NewEnumerator0
                                  (switch int _option_index__39
                                    (:0
                                      (bind (_state_40 _option_index__40) (CallFunction|AddDialogue "Encyclopaedia" "[Impossible:Fail] - \"Wow, Parsec, that's even shocked me, I have no idea what It means though, I'm sure you got it right though\"" (Utilities|Array|MakeArray "[LEAVE]")))
                                      (switch Utilities|FlowControl|Switch|SwitchonE_DialogueBase _state_40
                                        (:NewEnumerator0
                                          (switch int _option_index__40
                                            (:0
                                              (CallFunction|CloseDialogue)
                                              (CallFunction|CloseDialogue))))))
                                    (:1
                                      (CallFunction|ClearDialogueProgress)
                                      (CallFunction|CloseDialogue))))))))))))))))))
    (:1
      (bind (_state_41 _option_index__41) (CallFunction|AddDialogue "The Hooded Figure " "Ahh... So you've changed your mind? No worries, I understand... it is a hefty task" (Utilities|Array|MakeArray "\"Yes... I've changed my mind, please continue\"" "\"No I haven't changed my mind in fact\"")))
      (switch Utilities|FlowControl|Switch|SwitchonE_DialogueBase _state_41
        (:NewEnumerator0
          (switch int _option_index__41
            (:1
              (CallFunction|ClearDialogueProgress)
              (CallFunction|CloseDialogue))))))))
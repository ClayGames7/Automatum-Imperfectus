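; Dialogue component for the apartment's picture frame, where skill voices such as Perception, Logic and Half Light comment on a damaged photo of the player character.
; Overrides Dialogue, switching on DialogueTreeIndex into chained AddDialogue nodes that branch on the chosen option.
; Some endings set the index to select a follow-up tree for the revisited or smashed frame.
; Skill checks, morale changes and the thought gain appear only as text, with no logic behind them.
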(event EventBeginPlay
  (|CallParentFunction) ; This node is disabled and will not be called.\nDrag off pins to build functionality.
)

(event EventTick
  (params (DeltaSeconds :type Float%20%28single-precision%29))
  (|CallParentFunction DeltaSeconds) ; This node is disabled and will not be called.\nDrag off pins to build functionality.
)

(fn Dialogue
  (|CallParentFunction)
  (switch int (Variables|Default|GetDialogue%20Tree%20Index)
    (:0
      (bind (_state _option_index_) (CallFunction|AddDialogue "Picture Frame" "It's a cracked photo of a person in an old frame, it Looks Pre-Rennaisance era." (Utilities|Array|MakeArray "")))
      (switch Utilities|FlowControl|Switch|SwitchonE_DialogueBase _state
        (:NewEnumerator0
          (switch int _option_index_
            (:0
              (bind (_state_2 _option_index__2) (CallFunction|AddDialogue "Perception (Sight)" "[Heroic:Success] - A Hench and handsome young man in a trench coat and fedora with a missing Right arm" (Utilities|Array|MakeArray "")))
              (switch Utilities|FlowControl|Switch|SwitchonE_DialogueBase _state_2
                (:NewEnumerator0
                  (switch int _option_index__2
                    (:0
                      (bind (_state_3 _option_index__3) (CallFunction|AddDialogue "Esperit De Corps" "(if passed perception check) [Heroic:Success] - It's heavily damaged but you can see a Trench Coat and fedora, the classic siloheutte of a P.I or a detective, Used to counter the banging rain in this city, and these people have to explore outside for hours at a time" (Utilities|Array|MakeArray "")))
                      (switch Utilities|FlowControl|Switch|SwitchonE_DialogueBase _state_3
                        (:NewEnumerator0
                          (switch int _option_index__3
                            (:0
                              (bind (_state_4 _option_index__4) (CallFunction|AddDialogue "Logic" "(only if succeeding both checks) - A photo frame in our bedroom, wearing similar clothes to what we are now, This is clearly you." (Utilities|Array|MakeArray "1. - Needs a new frame, it's so broken." "2. - It's nothing, just a paperweight at this point (leave)" "3. (if passed checks) - Wow I looked good, What happened to me?")))
                              (switch Utilities|FlowControl|Switch|SwitchonE_DialogueBase _state_4
                                (:NewEnumerator0
                                  (switch int _option_index__4
                                    (:0
                                      (bind (_state_5 _option_index__5) (CallFunction|AddDialogue "Physical Instrument" "It's beautifully broken, must've taken some strong force to do this... I'm in awe." (Utilities|Array|MakeArray "")))
                                      (switch Utilities|FlowControl|Switch|SwitchonE_DialogueBase _state_5
                                        (:NewEnumerator0
                                          (switch int _option_index__5
                                            (:0
                                              (bind (_state_6 _option_index__6) (CallFunction|AddDialogue "Half Light" "DAMN IT'S NOT BROKEN ENOUGH!!! BREAK IT NOW!" (Utilities|Array|MakeArray "")))
                                              (switch Utilities|FlowControl|Switch|SwitchonE_DialogueBase _state_6
                                                (:NewEnumerator0
                                                  (switch int _option_index__6
                                                    (:0
                                                      (bind (_state_7 _option_index__7) (CallFunction|AddDialogue "Volition" "I advise you not to do that." (Utilities|Array|MakeArray "1. - No, I don't think destroying more things will help anyone. (LEAVE)" "2. - [Half Light - Medium 12] LOB THE PICTURE AT THE WALL")))
                                                      (switch Utilities|FlowControl|Switch|SwitchonE_DialogueBase _state_7
                                                        (:NewEnumerator0
                                                          (switch int _option_index__7
                                                            (:0
                                                              (CallFunction|RemoveDialogueProgress 3)
                                                              (CallFunction|CloseDialogue))
                                                            (:1
                                                              (switch Utilities|FlowControl|Switch|SwitchonE_DialogueBase "NewEnumerator0"
                                                                (:NewEnumerator0
                                                                  (switch int 0
                                                                    (:0
                                                                      (bind (_state_8 _option_index__8) (CallFunction|AddDialogue "Half Light" "[Medium:Success] - The picture is thrown so fast at the wall, how do you do it? Like a Blazeballer the frame breaks mach speed flying to the wall, until... CRACK, and the frame breaks into thousands of pieces" (Utilities|Array|MakeArray "")))
                                                                      (switch Utilities|FlowControl|Switch|SwitchonE_DialogueBase _state_8
                                                                        (:NewEnumerator0
                                                                          (switch int _option_index__8
                                                                            (:0
                                                                              (bind (_state_9 _option_index__9) (CallFunction|AddDialogue "Half Light" "Half Light - WE DID SO GOOD! I LOVED THAT BREAKING STUFF LIKE BISCUITS UNTIL THEY'RE LIMP AND DESTROYED! 
Thought Gained - Break Stuff" (Utilities|Array|MakeArray "Leave")))
                                                                              (switch Utilities|FlowControl|Switch|SwitchonE_DialogueBase _state_9
                                                                                (:NewEnumerator0
                                                                                  (switch int _option_index__9
                                                                                    (:0
                                                                                      (CallFunction|SetDialogueTreeIndex 2)
                                                                                      (CallFunction|CloseDialogue))))))))))))))))))))))))))
                                    (:1
                                      (CallFunction|RemoveDialogueProgress)
                                      (CallFunction|CloseDialogue))
                                    (:2
                                      (bind (_state_10 _option_index__10) (CallFunction|AddDialogue "Physical Instrument" "You have gotten absolutely huge, a stretegic bulk I say, the Cut will be incredible, Look at the muscles" (Utilities|Array|MakeArray "")))
                                      (switch Utilities|FlowControl|Switch|SwitchonE_DialogueBase _state_10
                                        (:NewEnumerator0
                                          (switch int _option_index__10
                                            (:0
                                              (bind (_state_11 _option_index__11) (CallFunction|AddDialogue "Perception (Sight)" "You have no muscles, no clear sign of the gym." (Utilities|Array|MakeArray "")))
                                              (switch Utilities|FlowControl|Switch|SwitchonE_DialogueBase _state_11
                                                (:NewEnumerator0
                                                  (switch int _option_index__11
                                                    (:0
                                                      (bind (_state_12 _option_index__12) (CallFunction|AddDialogue "Pain Threshold" "Pain threshold (If you failed the overhead kick) - Look at what you just managed to fail at, You failed to kick a ball because you are so unfit.  
NEGATIVE 1 MORALE" (Utilities|Array|MakeArray "")))
                                                      (switch Utilities|FlowControl|Switch|SwitchonE_DialogueBase _state_12
                                                        (:NewEnumerator0
                                                          (switch int _option_index__12
                                                            (:0
                                                              (bind (_state_13 _option_index__13) (CallFunction|AddDialogue "Volition" " Ignore them, You are still young, healthy and You have to believe in yourself or else we cannot find who we really are.  
HEALED MORALE +1" (Utilities|Array|MakeArray "")))
                                                              (switch Utilities|FlowControl|Switch|SwitchonE_DialogueBase _state_13
                                                                (:NewEnumerator0
                                                                  (switch int _option_index__13
                                                                    (:0
                                                                      (bind (_state_14 _option_index__14) (CallFunction|AddDialogue "Empathy" "It's best to leave now" (Utilities|Array|MakeArray "(Leave)")))
                                                                      (switch Utilities|FlowControl|Switch|SwitchonE_DialogueBase _state_14
                                                                        (:NewEnumerator0
                                                                          (switch int _option_index__14
                                                                            (:0
                                                                              (CallFunction|SetDialogueTreeIndex 1)
                                                                              (CallFunction|CloseDialogue))))))))))))))))))))))))))))))))))))))
    (:1
      (bind (_state_15 _option_index__15) (CallFunction|AddDialogue "Picture Frame" "There is no reason to torture yourself with this memento anymore" (Utilities|Array|MakeArray "")))
      (switch Utilities|FlowControl|Switch|SwitchonE_DialogueBase _state_15
        (:NewEnumerator0
          (switch int _option_index__15
            (:0
              (CallFunction|ClearDialogueProgress)
              (CallFunction|CloseDialogue))))))
    (:2
      (bind (_state_16 _option_index__16) (CallFunction|AddDialogue "Broken Picture Frame" "A shattered cropse lays at your feet, a victim of a murder." (Utilities|Array|MakeArray "")))
      (switch Utilities|FlowControl|Switch|SwitchonE_DialogueBase _state_16
        (:NewEnumerator0
          (switch int _option_index__16
            (:0
              (bind (_state_17 _option_index__17) (CallFunction|AddDialogue "Half Light" "AHAHAHA OHH IT IS BEAUTIFUL ISN'T IT" (Utilities|Array|MakeArray "Truly Beautiful... (Leave)")))
              (switch Utilities|FlowControl|Switch|SwitchonE_DialogueBase _state_17
                (:NewEnumerator0
                  (switch int _option_index__17
                    (:0
                      (CallFunction|ClearDialogueProgress)
                      (CallFunction|CloseDialogue))))))))))))
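; Dialogue component for the apartment's clothes pile, where skill voices such as Volition, Drama and Inland Empire speculate on whose clothes these are.
; The overridden Dialogue function switches on DialogueTreeIndex and chains AddDialogue calls, with skill check results written directly into the text.
; The first tree ends in a choice to accept a task or leave, which only sets the tree index for the matching short repeat line.
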(event EventBeginPlay
  (|CallParentFunction) ; This node is disabled and will not be called.\nDrag off pins to build functionality.
)

(event EventTick
  (params (DeltaSeconds :type Float%20%28single-precision%29))
  (|CallParentFunction DeltaSeconds) ; This node is disabled and will not be called.\nDrag off pins to build functionality.
)

(fn Dialogue
  (|CallParentFunction)
  (switch int (Variables|Default|GetDialogue%20Tree%20Index)
    (:0
      (bind (_state _option_index_) (CallFunction|AddDialogue "Clothes Pile" "A horribly messy bed, looks like a pigsty. Perhaps the only Pigsty left in this city" (Utilities|Array|MakeArray "")))
      (switch Utilities|FlowControl|Switch|SwitchonE_DialogueBase _state
        (:NewEnumerator0
          (switch int _option_index_
            (:0
              (bind (_state_2 _option_index__2) (CallFunction|AddDialogue "Volition" "This is not the consequences of a depressed man, which wouldn't have suprised anyone. But these clothes... they aren't yours." (Utilities|Array|MakeArray "")))
              (switch Utilities|FlowControl|Switch|SwitchonE_DialogueBase _state_2
                (:NewEnumerator0
                  (switch int _option_index__2
                    (:0
                      (bind (_state_3 _option_index__3) (CallFunction|AddDialogue "Visual Calculus" "But whose are they?" (Utilities|Array|MakeArray "")))
                      (switch Utilities|FlowControl|Switch|SwitchonE_DialogueBase _state_3
                        (:NewEnumerator0
                          (switch int _option_index__3
                            (:0
                              (bind (_state_4 _option_index__4) (CallFunction|AddDialogue "Conceptualisation" "A scorned lover who came and thrashed our room to the pits, a revenge on our scandelous acts, perhaps why we have lost our memory" (Utilities|Array|MakeArray "")))
                              (switch Utilities|FlowControl|Switch|SwitchonE_DialogueBase _state_4
                                (:NewEnumerator0
                                  (switch int _option_index__4
                                    (:0
                                      (bind (_state_5 _option_index__5) (CallFunction|AddDialogue "Drama" "[Easy:Success] - They doth lie, m'lord, Thou hath never had a lover, just you and us." (Utilities|Array|MakeArray "")))
                                      (switch Utilities|FlowControl|Switch|SwitchonE_DialogueBase _state_5
                                        (:NewEnumerator0
                                          (switch int _option_index__5
                                            (:0
                                              (bind (_state_6 _option_index__6) (CallFunction|AddDialogue "Electrochemistry" "[Medium:Success] - AND A BIG BOTTLE O' SYNTH IN YOUR HAND" (Utilities|Array|MakeArray "")))
                                              (switch Utilities|FlowControl|Switch|SwitchonE_DialogueBase _state_6
                                                (:NewEnumerator0
                                                  (switch int _option_index__6
                                                    (:0
                                                      (bind (_state_7 _option_index__7) (CallFunction|AddDialogue "Inland Empire" "You just know you will find this mystery out, it's not just a hunch you feel, the creaking of the ventys seem to call out to a wormhole in time... It is only a game of patience." (Utilities|Array|MakeArray "1. - Wow... I can feel everything pointing me to the future, This is new, I wonder what this is. (ACCEPT TASK)" "2. - It's just a pair of clothes, I'm thinking too much into this (LEAVE)")))
                                                      (switch Utilities|FlowControl|Switch|SwitchonE_DialogueBase _state_7
                                                        (:NewEnumerator0
                                                          (switch int _option_index__7
                                                            (:0
                                                              (bind (_state_8 _option_index__8) (CallFunction|AddDialogue "Inland Empire" "This is the only way to have done this, you Won't regret it." (Utilities|Array|MakeArray "")))
                                                              (switch Utilities|FlowControl|Switch|SwitchonE_DialogueBase _state_8
                                                                (:NewEnumerator0
                                                                  (switch int _option_index__8
                                                                    (:0
                                                                      (bind (_state_9 _option_index__9) (CallFunction|AddDialogue "Logic" "[Hard:Success] - There is no such thing as a wormhole, and the air vents are not speaking to us. You are just coming back from retrograde amnesia and going crazy." (Utilities|Array|MakeArray "Leave")))
                                                                      (switch Utilities|FlowControl|Switch|SwitchonE_DialogueBase _state_9
                                                                        (:NewEnumerator0
                                                                          (switch int _option_index__9
                                                                            (:0
                                                                              (CallFunction|SetDialogueTreeIndex 2)
                                                                              (CallFunction|CloseDialogue))))))))))
                                                            (:1
                                                              (CallFunction|SetDialogueTreeIndex 1)
                                                              (CallFunction|CloseDialogue))))))))))))))))))))))))))))))
    (:1
      (bind (_state_10 _option_index__10) (CallFunction|AddDialogue "Clothes Pile" "Just a plain old mess of clothes" (Utilities|Array|MakeArray "(Leave)")))
      (switch Utilities|FlowControl|Switch|SwitchonE_DialogueBase _state_10
        (:NewEnumerator0
          (switch int _option_index__10
            (:0
              (CallFunction|ClearDialogueProgress)
              (CallFunction|CloseDialogue))))))
    (:2
      (bind (_state_11 _option_index__11) (CallFunction|AddDialogue "Inland Empire" "Patience is a virtue, you will find the wormhole..." (Utilities|Array|MakeArray "(Leave)")))
      (switch Utilities|FlowControl|Switch|SwitchonE_DialogueBase _state_11
        (:NewEnumerator0
          (switch int _option_index__11
            (:0
              (CallFunction|ClearDialogueProgress)
              (CallFunction|CloseDialogue))))))))
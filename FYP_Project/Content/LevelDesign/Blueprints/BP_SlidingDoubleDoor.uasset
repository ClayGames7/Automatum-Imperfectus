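; Sliding double door that toggles between open and closed each time it receives an Interact event.
; A Sequence fires two FlipFlops, one per panel, which alternately play and reverse that panel's Timeline.
; Each Timeline track drives a Lerp on the panel's relative Y location, sliding the two panels apart in opposite directions.
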(event EventInteract
  (params (Instigator :type Actor%20Object%20Reference))
  (Utilities|FlowControl|Sequence
    (:then_0
      (Utilities|FlowControl|FlipFlop
        (:A
          (bind _doortrack (Timeline|Left%20door%20open Play)
            (:Update
              (Transformation|SetRelativeLocation (Variables|Default|GetLeft%20Door) (Math|Vector|MakeVector 0.0 (Math|Float|Lerp 0.0 -1.2e+02 _doortrack) 0.0) false false))))
        (:B
          (Timeline|Left%20door%20open Reverse))))
    (:then_1
      (Utilities|FlowControl|FlipFlop
        (:A
          (bind _doortrack_2 (Timeline|Right%20Door%20Open Play)
            (:Update
              (Transformation|SetRelativeLocation (Variables|Default|GetRight%20Door) (Math|Vector|MakeVector 0.0 (Math|Float|Lerp 0.0 1.2e+02 _doortrack_2) 0.0) false false))))
        (:B
          (Timeline|Right%20Door%20Open Reverse))))))

(fn ConstructionScript)